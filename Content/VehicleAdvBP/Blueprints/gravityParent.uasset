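; gravityParent is a gravity-body actor Blueprint whose logic is unwired: BeginPlay runs an empty loop and Tick does nothing.
; Disconnected graphs would pull it toward other gravityParent actors with inverse-square velocity additions, and spawn and attach 100 PowerPellets around it.
; CreateCircle supplies flat spawn offsets from separately randomized sine and cosine angles, so points scatter across a square rather than tracing a circle.
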(event `self.ReceiveBeginPlay`
  (for _ (range 5)
    _))

(event `self.ReceiveTick`
  (params (DeltaSeconds :type "Float (single-precision)")))

(fn `createCircle`
  (params (NewParam1 :type "Float (double-precision)"))
  (returns (NewParam :type "Vector Structure"))
  (bind _returnvalue (`KismetMathLibrary.RandomFloatInRange` -360.0 360.0))
  (return (`KismetMathLibrary.MakeVector` (* NewParam1 (`KismetMathLibrary.DegSin` _returnvalue)) (* NewParam1 (`KismetMathLibrary.DegCos` _returnvalue)))))

(fn `UserConstructionScript`)