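; Level clock actor that counts elapsed game seconds and ends the game when time runs out.
; BeginPlay caches the rollingStarInstance GameInstance and clears its TimeEnd flag, leaving the Seconds count as it is.
; Tick feeds a one-second Delay that increments Seconds and sets TimeEnd once it reaches TotalSeconds.
; When TimeEnd is set, Tick opens the "end" level.
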(event `self.ReceiveTick`
  (params (DeltaSeconds :type "Float (single-precision)"))
  (if (`/Game/VehicleAdvBP/Blueprints/rollingStarInstance.timeEnd` (`self.GameInst`))
    (`GameplayStatics.OpenLevel` "end")
    (else
      (`KismetSystemLibrary.Delay` 1.0)
      (bind _result (`/Engine/EditorBlueprintResources/StandardMacros.IncrementInt` (`/Game/VehicleAdvBP/Blueprints/rollingStarInstance.seconds` (`self.GameInst`)))
        (:`  `
          (bind _output_get (set `/Game/VehicleAdvBP/Blueprints/rollingStarInstance.seconds` _result (`self.GameInst`)))
          (if (not (< _output_get (`/Game/VehicleAdvBP/Blueprints/rollingStarInstance.totalSeconds` (`self.GameInst`))))
            (set `/Game/VehicleAdvBP/Blueprints/rollingStarInstance.timeEnd` true (`self.gameInst`))))))))

(event `self.ReceiveBeginPlay`
  (bind _output_get (set `self.GameInst` (cast `/Game/VehicleAdvBP/Blueprints/rollingStarInstance` (`GameplayStatics.GetGameInstance`) :!pure true)))
  (set `/Game/VehicleAdvBP/Blueprints/rollingStarInstance.timeEnd` false _output_get))

(fn `UserConstructionScript`)