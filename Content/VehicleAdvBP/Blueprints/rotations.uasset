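; Blueprint helper graphs in the VehicleAdvBP project that compute coordinates for circular motion.
; RotSin and RotCos take the degree-based sine or cosine of an angle over a divisor, scaled by an amplitude.
; Rotation adds a step to the angle, feeds it to both for X and Y, sets Z to a quarter of the amplitude and also returns the advanced angle.
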(fn `rotation`
  (params (A :type "Float (double-precision)") (B :type "Float (double-precision)") (InputPin :type "Float (double-precision)") (B1 :type "Float (double-precision)"))
  (returns (NewParam :type "Vector Structure") (Result :type "Float (double-precision)"))
  (bind _returnvalue (+ A B1))
  (bind _returnvalue_2 (`self.rotSin` null _returnvalue B InputPin))
  (bind _returnvalue_3 (`self.rotCos` null _returnvalue B InputPin))
  (return (`KismetMathLibrary.MakeVector` _returnvalue_2 _returnvalue_3 (/ InputPin 4.0)) _returnvalue))

(fn `rotCos`
  (params (A :type "Float (double-precision)") (B :type "Float (double-precision)") (InputPin :type "Float (double-precision)"))
  (returns (ReturnValue :type "Float (double-precision)"))
  (return (* (`KismetMathLibrary.DegCos` (/ A B)) InputPin)))

(fn `rotSin`
  (params (A :type "Float (double-precision)") (B :type "Float (double-precision)") (InputPin :type "Float (double-precision)"))
  (returns (ReturnValue :type "Float (double-precision)"))
  (return (* (`KismetMathLibrary.DegSin` (/ A B)) InputPin)))