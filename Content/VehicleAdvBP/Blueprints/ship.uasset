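; Ship actor Blueprint that appears to be an unfinished prototype for movement around a GravityParent body.
; On BeginPlay it caches the first GravityParent found; Tick, overlap, movement inputs and construction script are empty.
; Disconnected, never-executed experiments remain: trace-based height correction through physics velocity, orbit-style rotation, and orientation using the direction away from the gravity actor.
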(event `InputAxis|MoveRight`
  (params (AxisValue :type "Float (single-precision)")))

(event `self.ReceiveActorBeginOverlap`
  (params (OtherActor :type "Actor Object Reference")))

(event `self.ReceiveBeginPlay`
  (bind _outactors (`GameplayStatics.GetAllActorsOfClass` "/Game/VehicleAdvBP/Blueprints/gravityParent.gravityParent_C"))
  (set `self.NewVar_1` (`|GetArrayItem` _outactors)))

(event `self.ReceiveTick`
  (params (DeltaSeconds :type "Float (single-precision)")))

(event `InputAxis|MoveForward`
  (params (AxisValue :type "Float (single-precision)")))

(fn `UserConstructionScript`)